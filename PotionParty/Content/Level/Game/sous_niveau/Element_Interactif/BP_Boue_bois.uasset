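; Interactive level element, described as a boat in its comment, that moves its static mesh along a spline path on a repeating cycle.
; BeginPlay starts a timeline whose TravelDistance track, scaled by spline length, sets the mesh's world location without sweep or rotation.
; Looping comes from a fixed Delay on the timeline's Update pin, which calls Start again, rather than from the Finished pin or timeline looping.
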(event `self.ReceiveBeginPlay`
  ;[1 1 1] Fais suivre la tragectoire au bateau grace a une animation de déplacement
  (`self.Start`))

(event `Start`
  ;[1 1 1] Fais suivre la tragectoire au bateau grace a une animation de déplacement
  (bind (_direction _traveldistance) (`Timeline|MovingLibrary` :!via `PlayFromStart`)
    (:`Update`
      (`SceneComponent.K2_SetWorldLocation` (`self.StaticMesh`) (`SplineComponent.GetLocationAtDistanceAlongSpline` (`self.Spline`) (* _traveldistance (`SplineComponent.GetSplineLength` (`self.Spline`))) "World") false false)
      (`KismetSystemLibrary.Delay` 11.0)
      (`self.Start`))))

(fn `UserConstructionScript`)