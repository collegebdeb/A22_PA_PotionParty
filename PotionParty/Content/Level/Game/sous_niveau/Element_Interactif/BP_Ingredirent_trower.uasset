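; Test spawner actor that periodically throws random ingredients into the level from inside its Box extent.
; Tremblement starts on BeginPlay, waits through a fixed Delay, spawns a batch sized by Nombre, then calls itself to repeat.
; Nested coin flips choose berry, throwing ingredient, rat tail or ectoplasm at random box points.
; Only berries and throwing ingredients receive a randomized launch impulse, biased toward +Y and upward.
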(event `self.ReceiveBeginPlay`
  ;[1 1 1] Fait spawn des ingrédient a 5 seonde et ensuite a chaque 10 seconde (Juste un test)
  (`self.Tremblement`))

(event `Tremblement`
  (bind _returnvalue (`KismetMathLibrary.RandomPointInBoundingBox` (`SceneComponent.K2_GetComponentLocation` (`self.DefaultSceneRoot`)) (`BoxComponent.GetScaledBoxExtent` (`self.Box`))))
  ;[1 1 1] Fait spawn des ingrédient a 5 seonde et ensuite a chaque 10 seconde (Juste un test)
  (`KismetSystemLibrary.Delay` 10.0)
  (for _ (range (+ (`self.Nombre`) 1))
    (if (`KismetMathLibrary.RandomBool`)
      (if (`KismetMathLibrary.RandomBool`)
        (bind _returnvalue_2 (`|SpawnActorFromClass` "/Game/Blueprint/BP_Baie_sol.BP_Baie_sol_C" (`KismetMathLibrary.MakeTransform` _returnvalue) "Undefined" "OverrideRootScale" null null))
        (`PrimitiveComponent.AddImpulse` (`/Game/Blueprint/BP_Baie_sol.Baie` _returnvalue_2) (`KismetMathLibrary.MakeVector` (`KismetMathLibrary.RandomFloatInRange` -500.0 500.0) (`KismetMathLibrary.RandomFloatInRange` 700.0 1800.0) (`KismetMathLibrary.RandomFloatInRange` 700.0 2000.0)) "None" false)
        (else
          (bind _returnvalue_3 (`|SpawnActorFromClass` "/Game/Level/Game/sous_niveau/Element_Interactif/BP_Trowing_ingredient.BP_Trowing_ingredient_C" (`KismetMathLibrary.MakeTransform` _returnvalue) "Undefined" "OverrideRootScale" null null))
          (`PrimitiveComponent.AddImpulse` (`/Game/Level/Game/sous_niveau/Element_Interactif/BP_Trowing_ingredient.Cube` _returnvalue_3) (`KismetMathLibrary.MakeVector` (`KismetMathLibrary.RandomFloatInRange` -500.0 500.0) (`KismetMathLibrary.RandomFloatInRange` 700.0 1800.0) (`KismetMathLibrary.RandomFloatInRange` 700.0 2000.0)) "None" false)))
      (elif (`KismetMathLibrary.RandomBool`)
        (`|SpawnActorFromClass` "/Game/Level/Game/sous_niveau/Element_Interactif/Special_ingredient/BP_queueDeRat_sol_Jousting.BP_queueDeRat_sol_Jousting_C" (`KismetMathLibrary.MakeTransform` _returnvalue) "Undefined" "OverrideRootScale" null null)
        (else
          (`|SpawnActorFromClass` "/Game/Level/Game/sous_niveau/Element_Interactif/Special_ingredient/BP_Ectoplasme_sol_jousting.BP_Ectoplasme_sol_jousting_C" (`KismetMathLibrary.MakeTransform` _returnvalue) "Undefined" "OverrideRootScale" null null)))))
  (`self.Tremblement`))

(fn `UserConstructionScript`)