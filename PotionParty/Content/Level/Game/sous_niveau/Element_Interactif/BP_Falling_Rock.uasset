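; BP_Falling_Rock is a falling rock hazard that damages the player and shows a shadow that scales with its height.
; Each tick it finds a Ground_point actor and scales Ombre on Y and Z by the ratio of that point's height to the Sphere's.
; A Sphere overlap with ThirdPersonCharacter calls TakeDamage and destroys the rock immediately.
; A hit on any of its three Cube components destroys it after a short delay.
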(event `self.ReceiveBeginPlay`)

(event `self.ReceiveTick`
  (params (DeltaSeconds :type "Float (single-precision)"))
  (bind (_returnvalue_x _returnvalue_y _returnvalue_z) (`KismetMathLibrary.BreakVector` (`SceneComponent.K2_GetComponentLocation` (`self.Sphere`))))
  ;[1 1 1] En fonction de la distance avec le ground point fais grossir l'ombre
  (`/Engine/EditorBlueprintResources/StandardMacros.DoOnce` false :!label _label
    (:`Completed`
      (bind _returnvalue (`GameplayStatics.GetActorOfClass` "/Game/Level/Game/sous_niveau/Element_Interactif/Ground_point.Ground_point_C"))
      (bind (_returnvalue_x_2 _returnvalue_y_2 _returnvalue_z_2) (`KismetMathLibrary.BreakVector` (`SceneComponent.K2_GetComponentLocation` (`/Game/Level/Game/sous_niveau/Element_Interactif/Ground_point.DefaultSceneRoot` _returnvalue))))
      (bind _returnvalue_2 (* (/ _returnvalue_z_2 _returnvalue_z) 2.0))
      (`SceneComponent.SetRelativeScale3D` (`self.ombre`) (`KismetMathLibrary.MakeVector` 9.0 _returnvalue_2 _returnvalue_2))
      (goto _label :!via `Reset`))))

(event `self.Sphere.OnComponentBeginOverlap`
  (params (OverlappedComponent :type "PrimitiveComponent Object Reference") (OtherActor :type "Actor Object Reference") (OtherComp :type "PrimitiveComponent Object Reference") (OtherBodyIndex :type Integer) (bFromSweep :type Boolean) (SweepResult :type "HitResult Structure (by ref)"))
  ;[1 1 1] S'il entre en contacte avec le joueur lui fait prendre un dégat et se détruit, s'il touche le sol le détruit
  (bind _asthird_person_character (cast `/Game/ThirdPersonBP/Blueprints/ThirdPersonCharacter` OtherActor))
  (`/Game/ThirdPersonBP/Blueprints/ThirdPersonCharacter.TakeDamage` _asthird_person_character)
  (`self.K2_DestroyActor`))

(event `self.Cube.OnComponentHit`
  (params (HitComponent :type "PrimitiveComponent Object Reference") (OtherActor :type "Actor Object Reference") (OtherComp :type "PrimitiveComponent Object Reference") (NormalImpulse :type "Vector Structure") (Hit :type "HitResult Structure (by ref)"))
  ;[1 1 1] S'il entre en contacte avec le joueur lui fait prendre un dégat et se détruit, s'il touche le sol le détruit
  (`KismetSystemLibrary.Delay` 0.3 :!label _label_2)
  (`self.K2_DestroyActor`))

(event `self.Cube1.OnComponentHit`
  (params (HitComponent :type "PrimitiveComponent Object Reference") (OtherActor :type "Actor Object Reference") (OtherComp :type "PrimitiveComponent Object Reference") (NormalImpulse :type "Vector Structure") (Hit :type "HitResult Structure (by ref)"))
  ;[1 1 1] S'il entre en contacte avec le joueur lui fait prendre un dégat et se détruit, s'il touche le sol le détruit
  (goto _label_2))

(event `self.Cube2.OnComponentHit`
  (params (HitComponent :type "PrimitiveComponent Object Reference") (OtherActor :type "Actor Object Reference") (OtherComp :type "PrimitiveComponent Object Reference") (NormalImpulse :type "Vector Structure") (Hit :type "HitResult Structure (by ref)"))
  ;[1 1 1] S'il entre en contacte avec le joueur lui fait prendre un dégat et se détruit, s'il touche le sol le détruit
  (goto _label_2))

(fn `UserConstructionScript`)