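; Ingredient thrower actor (left-side variant, per its name) that periodically launches physics ingredient pickups into the level.
; After an initial delay on BeginPlay, the Tremblement event waits a random few seconds, spawns a Nombre-driven batch, then calls itself to repeat indefinitely.
; Nested random branches pick berry, mushroom, ectoplasm or rat tail with equal odds.
; Each spawns at a random point in the Box extent and gets a randomized +X, upward velocity.
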(event `self.ReceiveBeginPlay`
  ;[1 1 1] Fait spawn des ingrédient a 5 seonde et ensuite a chaque 10 seconde (Juste un test)
  (`KismetSystemLibrary.Delay` (`self.Delay`))
  (`self.Tremblement`))

(event `Tremblement`
  (bind _returnvalue (`KismetMathLibrary.RandomPointInBoundingBox` (`SceneComponent.K2_GetComponentLocation` (`self.DefaultSceneRoot`)) (`BoxComponent.GetScaledBoxExtent` (`self.Box`))))
  ;[1 1 1] Fait spawn des ingrédient a 5 seonde et ensuite a chaque 10 seconde (Juste un test)
  (`KismetSystemLibrary.Delay` (`KismetMathLibrary.RandomFloatInRange` 4.0 8.0))
  (for _ (range (+ (`self.Nombre`) 1))
    (if (`KismetMathLibrary.RandomBool`)
      (if (`KismetMathLibrary.RandomBool`)
        (bind _returnvalue_2 (`|SpawnActorFromClass` "/Game/Blueprint/BP_Baie_sol.BP_Baie_sol_C" (`KismetMathLibrary.MakeTransform` _returnvalue) "Undefined" "OverrideRootScale" null null))
        (`PrimitiveComponent.SetPhysicsLinearVelocity` (`/Game/Blueprint/BP_Baie_sol.Baie` _returnvalue_2) (`KismetMathLibrary.MakeVector` (`KismetMathLibrary.RandomFloatInRange` 700.0 1000.0) (`KismetMathLibrary.RandomFloatInRange` -200.0 200.0) (`KismetMathLibrary.RandomFloatInRange` 200.0 600.0)) false "None")
        (else
          (bind _returnvalue_3 (`|SpawnActorFromClass` "/Game/Blueprint/BP_Champignon_sol.BP_Champignon_sol_C" (`KismetMathLibrary.MakeTransform` _returnvalue) "Undefined" "OverrideRootScale" null null))
          (`PrimitiveComponent.SetPhysicsLinearVelocity` (`/Game/Blueprint/BP_Champignon_sol.champignon` _returnvalue_3) (`KismetMathLibrary.MakeVector` (`KismetMathLibrary.RandomFloatInRange` 700.0 1000.0) (`KismetMathLibrary.RandomFloatInRange` -200.0 200.0) (`KismetMathLibrary.RandomFloatInRange` 200.0 600.0)) false "None")))
      (elif (`KismetMathLibrary.RandomBool`)
        (bind _returnvalue_4 (`|SpawnActorFromClass` "/Game/Blueprint/BP_Ectoplasme_sol.BP_Ectoplasme_sol_C" (`KismetMathLibrary.MakeTransform` _returnvalue) "Undefined" "OverrideRootScale" null null))
        (`PrimitiveComponent.SetPhysicsLinearVelocity` (`/Game/Blueprint/BP_Ectoplasme_sol.ectoplasme` _returnvalue_4) (`KismetMathLibrary.MakeVector` (`KismetMathLibrary.RandomFloatInRange` 700.0 1000.0) (`KismetMathLibrary.RandomFloatInRange` -200.0 200.0) (`KismetMathLibrary.RandomFloatInRange` 200.0 600.0)) false "None")
        (else
          (bind _returnvalue_5 (`|SpawnActorFromClass` "/Game/Blueprint/BP_queueDeRat_sol.BP_queueDeRat_sol_C" (`KismetMathLibrary.MakeTransform` _returnvalue) "Undefined" "OverrideRootScale" null null))
          (`PrimitiveComponent.SetPhysicsLinearVelocity` (`/Game/Blueprint/BP_queueDeRat_sol.queue de rat` _returnvalue_5) (`KismetMathLibrary.MakeVector` (`KismetMathLibrary.RandomFloatInRange` 700.0 1000.0) (`KismetMathLibrary.RandomFloatInRange` -200.0 200.0) (`KismetMathLibrary.RandomFloatInRange` 200.0 600.0)) false "None")))))
  (`self.Tremblement`))

(fn `UserConstructionScript`)