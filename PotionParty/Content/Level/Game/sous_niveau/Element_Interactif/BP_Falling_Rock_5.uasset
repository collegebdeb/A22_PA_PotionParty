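; BP_Falling_Rock_5 is a falling rock hazard that damages the player and destroys itself.
; Sphere overlap with ThirdPersonCharacter calls TakeDamage, then destroys the rock after a short delay.
; A Cube component hit also destroys it after a brief delay.
; Logic to scale the Ombre shadow from the height ratio between Ground_point and the rock is disconnected, so Tick does nothing.
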(event `self.ReceiveBeginPlay`)

(event `self.ReceiveTick`
  (params (DeltaSeconds :type "Float (single-precision)"))
  ;[1 1 1] En fonction de la distance avec le ground point fais grossir l'ombre
)

(event `self.Sphere.OnComponentBeginOverlap`
  (params (OverlappedComponent :type "PrimitiveComponent Object Reference") (OtherActor :type "Actor Object Reference") (OtherComp :type "PrimitiveComponent Object Reference") (OtherBodyIndex :type Integer) (bFromSweep :type Boolean) (SweepResult :type "HitResult Structure (by ref)"))
  ;[1 1 1] S'il entre en contacte avec le joueur lui fait prendre un dégat et se détruit, s'il touche le sol le détruit
  (bind _asthird_person_character (cast `/Game/ThirdPersonBP/Blueprints/ThirdPersonCharacter` OtherActor))
  (`/Game/ThirdPersonBP/Blueprints/ThirdPersonCharacter.TakeDamage` _asthird_person_character)
  (`KismetSystemLibrary.Delay` 0.2)
  (`self.K2_DestroyActor`))

(event `self.Cube.OnComponentHit`
  (params (HitComponent :type "PrimitiveComponent Object Reference") (OtherActor :type "Actor Object Reference") (OtherComp :type "PrimitiveComponent Object Reference") (NormalImpulse :type "Vector Structure") (Hit :type "HitResult Structure (by ref)"))
  ;[1 1 1] S'il entre en contacte avec le joueur lui fait prendre un dégat et se détruit, s'il touche le sol le détruit
  (`KismetSystemLibrary.Delay` 0.1)
  (`self.K2_DestroyActor`))

(fn `UserConstructionScript`)