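; BP_biblio is an interactive level element: a library mesh that moves back and forth along a spline, meant to rise and descend.
; After a configurable start delay on BeginPlay, one timeline plays forward and a second in reverse, each mapping its track to distance along the spline.
; Fixed delays chained from the timelines' Update pins trigger the reverse pass, then call Start again, looping indefinitely.
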(event `self.ReceiveBeginPlay`
  ;[1 1 1] Regarde s'il faut attendre avant de commencer
  (`KismetSystemLibrary.Delay` (`self.WaitStartTime`))
  (`self.Start`))

(event `Start`
  ;[1 1 1] Fait monter et descendre les biblio en fonction de l'animation
  (bind (_direction _traveldistance) (`Timeline|MovingLibrary` :!via `PlayFromStart`)
    (:`Update`
      (`SceneComponent.K2_SetWorldLocation` (`self.StaticMesh`) (`SplineComponent.GetLocationAtDistanceAlongSpline` (`self.Spline`) (* _traveldistance (`SplineComponent.GetSplineLength` (`self.Spline`))) "World") false false)
      (`KismetSystemLibrary.Delay` 6.0)
      (bind (_direction_2 _traveldistance_2) (`Timeline|Timeline_0` :!via `ReverseFromEnd`)
        (:`Update`
          (`SceneComponent.K2_SetWorldLocation` (`self.StaticMesh`) (`SplineComponent.GetLocationAtDistanceAlongSpline` (`self.Spline`) (* _traveldistance_2 (`SplineComponent.GetSplineLength` (`self.Spline`))) "World") false false)
          (`KismetSystemLibrary.Delay` 6.0)
          (`self.Start`))))))

(fn `UserConstructionScript`)