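; Level actor that repeatedly drops salvos of falling rocks from a box volume for as long as it is in play.
; BeginPlay waits a short random delay before the first salvo, then Tremblement calls itself to repeat the delay and salvo indefinitely.
; Each salvo spawns rocks according to Nombre, picking among four BP_Falling_Rock variants through nested random booleans, at random points inside the Box.
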(event `self.ReceiveBeginPlay`
  (bind _returnvalue (`KismetMathLibrary.RandomPointInBoundingBox` (`SceneComponent.K2_GetComponentLocation` (`self.DefaultSceneRoot`)) (`BoxComponent.GetScaledBoxExtent` (`self.Box`))))
  ;[1 1 1] Fait spawn une salve de roche a 15 seconde et ensuite a chaque 20 seconde
  (`KismetSystemLibrary.Delay` (`KismetMathLibrary.RandomFloatInRange` 5.0 10.0))
  (for _ (range (+ (`self.Nombre`) 1))
    (if (`KismetMathLibrary.RandomBool`) :!label _label
      (if (`KismetMathLibrary.RandomBool`)
        (`|SpawnActorFromClass` "/Game/Level/Game/sous_niveau/Element_Interactif/BP_Falling_Rock_2.BP_Falling_Rock_2_C" (`KismetMathLibrary.MakeTransform` _returnvalue) "Undefined" "OverrideRootScale" null null)
        (else
          (`|SpawnActorFromClass` "/Game/Level/Game/sous_niveau/Element_Interactif/BP_Falling_Rock_3.BP_Falling_Rock_3_C" (`KismetMathLibrary.MakeTransform` _returnvalue) "Undefined" "OverrideRootScale" null null)))
      (elif (`KismetMathLibrary.RandomBool`)
        (`|SpawnActorFromClass` "/Game/Level/Game/sous_niveau/Element_Interactif/BP_Falling_Rock_4.BP_Falling_Rock_4_C" (`KismetMathLibrary.MakeTransform` _returnvalue) "Undefined" "OverrideRootScale" null null)
        (else
          (`|SpawnActorFromClass` "/Game/Level/Game/sous_niveau/Element_Interactif/BP_Falling_Rock_5.BP_Falling_Rock_5_C" (`KismetMathLibrary.MakeTransform` _returnvalue) "Undefined" "OverrideRootScale" null null)))))
  (`self.Tremblement`))

(event `Tremblement`
  ;[1 1 1] Fait spawn une salve de roche a 15 seconde et ensuite a chaque 20 seconde
  (`KismetSystemLibrary.Delay` (`KismetMathLibrary.RandomFloatInRange` 5.0 10.0))
  (for _ (range (+ (`self.Nombre`) 1))
    (goto _label))
  (`self.Tremblement`))

(fn `UserConstructionScript`)