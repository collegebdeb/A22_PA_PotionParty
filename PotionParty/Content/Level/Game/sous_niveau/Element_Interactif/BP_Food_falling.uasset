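; BP_Food_falling is a level spawner that repeatedly scatters food actors inside a box volume.
; After an initial configurable delay, the Tremblement event waits a random 3 to 10 seconds, spawns a batch sized by Nombre, then calls itself to loop.
; Nested coin flips pick berry, mushroom, ectoplasm or rat tail ground actors, each placed at a random point within the box extent around the root.
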(event `self.ReceiveBeginPlay`
  (`KismetSystemLibrary.Delay` (`self.Delay`))
  (`self.Tremblement`))

(event `Tremblement`
  (bind _returnvalue (`KismetMathLibrary.RandomPointInBoundingBox` (`SceneComponent.K2_GetComponentLocation` (`self.DefaultSceneRoot`)) (`BoxComponent.GetScaledBoxExtent` (`self.Box`))))
  (`KismetSystemLibrary.Delay` (`KismetMathLibrary.RandomFloatInRange` 3.0 10.0))
  (for _ (range (+ (`self.Nombre`) 1))
    (if (`KismetMathLibrary.RandomBool`)
      (if (`KismetMathLibrary.RandomBool`)
        (`|SpawnActorFromClass` "/Game/Blueprint/BP_Baie_sol.BP_Baie_sol_C" (`KismetMathLibrary.MakeTransform` _returnvalue) "Undefined" "OverrideRootScale" null null)
        (else
          (`|SpawnActorFromClass` "/Game/Blueprint/BP_Champignon_sol.BP_Champignon_sol_C" (`KismetMathLibrary.MakeTransform` _returnvalue) "Undefined" "OverrideRootScale" null null)))
      (elif (`KismetMathLibrary.RandomBool`)
        (`|SpawnActorFromClass` "/Game/Blueprint/BP_Ectoplasme_sol.BP_Ectoplasme_sol_C" (`KismetMathLibrary.MakeTransform` _returnvalue) "Undefined" "OverrideRootScale" null null)
        (else
          (`|SpawnActorFromClass` "/Game/Blueprint/BP_queueDeRat_sol.BP_queueDeRat_sol_C" (`KismetMathLibrary.MakeTransform` _returnvalue) "Undefined" "OverrideRootScale" null null)))))
  (`self.Tremblement`))

(fn `UserConstructionScript`)