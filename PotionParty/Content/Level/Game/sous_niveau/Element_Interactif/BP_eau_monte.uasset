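; BP_eau_monte is an interactive level element that moves a static mesh back and forth along a spline, apparently rising water or a boat.
; After a random delay on BeginPlay, one timeline drives the mesh forward by spline distance, and a second, reversed timeline brings it back.
; Fixed delays chained from each timeline's Update, rather than Finished, trigger the return and restart the cycle.
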(event `self.ReceiveTick`
  (params (DeltaSeconds :type "Float (single-precision)")))

(event `Start`
  ;[1 1 1] Fais suivre la tragectoire au bateau grace a une animation de déplacement
  (`KismetSystemLibrary.Delay` (`KismetMathLibrary.RandomFloatInRange` 20.0 30.0))
  (bind (_direction _traveldistance) (`Timeline|MovingLibrary` :!via `PlayFromStart`)
    (:`Update`
      (`SceneComponent.K2_SetWorldLocation` (`self.StaticMesh`) (`SplineComponent.GetLocationAtDistanceAlongSpline` (`self.Spline`) (* _traveldistance (`SplineComponent.GetSplineLength` (`self.Spline`))) "World") false false)
      (`KismetSystemLibrary.Delay` 20.0)
      (bind (_direction_2 _traveldistance_2) (`Timeline|Timeline_0` :!via `ReverseFromEnd`)
        (:`Update`
          (`SceneComponent.K2_SetWorldLocation` (`self.StaticMesh`) (`SplineComponent.GetLocationAtDistanceAlongSpline` (`self.Spline`) (* _traveldistance_2 (`SplineComponent.GetSplineLength` (`self.Spline`))) "World") false false)
          (`KismetSystemLibrary.Delay` 11.0)
          (`self.Start`))))))

(event `self.ReceiveBeginPlay`
  ;[1 1 1] Fais suivre la tragectoire au bateau grace a une animation de déplacement
  (`self.Start`))

(fn `UserConstructionScript`)