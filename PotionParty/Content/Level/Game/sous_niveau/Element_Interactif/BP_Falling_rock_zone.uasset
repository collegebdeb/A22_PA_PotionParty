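; BP_Falling_rock_zone is a level zone actor that periodically spawns salvos of falling rocks.
; BeginPlay waits 15 seconds, then spawns BP_Falling_Rock actors at random points within the Box extent around the root, with the loop count set by Nombre.
; The Tremblement event then repeats the salvo indefinitely, calling itself after each 20-second delay and reusing the same spawn node.
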(event `self.ReceiveBeginPlay`
  ;[1 1 1] Fait spawn une salve de roche a 15 seconde et ensuite a chaque 20 seconde
  (`KismetSystemLibrary.Delay` 15.0)
  (for _ (range (+ (`self.Nombre`) 1))
    (`|SpawnActorFromClass` "/Game/Level/Game/sous_niveau/Element_Interactif/BP_Falling_Rock.BP_Falling_Rock_C" (`KismetMathLibrary.MakeTransform` (`KismetMathLibrary.RandomPointInBoundingBox` (`SceneComponent.K2_GetComponentLocation` (`self.DefaultSceneRoot`)) (`BoxComponent.GetScaledBoxExtent` (`self.Box`)))) "Undefined" "OverrideRootScale" null null :!label _label))
  (`self.Tremblement`))

(event `Tremblement`
  ;[1 1 1] Fait spawn une salve de roche a 15 seconde et ensuite a chaque 20 seconde
  (`KismetSystemLibrary.Delay` 20.0)
  (for _ (range (+ (`self.Nombre`) 1))
    (goto _label))
  (`self.Tremblement`))

(fn `UserConstructionScript`)