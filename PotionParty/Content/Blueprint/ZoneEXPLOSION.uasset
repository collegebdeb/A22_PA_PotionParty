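; Short-lived explosion zone actor that spawns an explosive ghost AI and hurts the player character.
; On BeginPlay it spawns IA_fantome_Explosive at a random point within its Box extent around the root, then prints a debug message and destroys itself after a short delay.
; While it exists, any ThirdPersonCharacter that begins overlapping its Sphere has TakeDamage called on it.
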(event `self.ReceiveBeginPlay`
  (`AIBlueprintHelperLibrary.SpawnAIFromClass` "/Game/ThirdPersonBP/IA/IA_fantome_Explosive.IA_fantome_Explosive_C" null (`KismetMathLibrary.RandomPointInBoundingBox` (`SceneComponent.K2_GetComponentLocation` (`self.DefaultSceneRoot`)) (`BoxComponent.BoxExtent` (`self.Box`))) (struct) false null)
  (`KismetSystemLibrary.Delay` 1.0)
  (`KismetSystemLibrary.PrintString` "Explosion")
  (`self.K2_DestroyActor`))

(event `self.Sphere.OnComponentBeginOverlap`
  (params (OverlappedComponent :type "PrimitiveComponent Object Reference") (OtherActor :type "Actor Object Reference") (OtherComp :type "PrimitiveComponent Object Reference") (OtherBodyIndex :type Integer) (bFromSweep :type Boolean) (SweepResult :type "HitResult Structure (by ref)"))
  (bind _asthird_person_character (cast `/Game/ThirdPersonBP/Blueprints/ThirdPersonCharacter` OtherActor))
  (`/Game/ThirdPersonBP/Blueprints/ThirdPersonCharacter.TakeDamage` _asthird_person_character))

(fn `UserConstructionScript`)