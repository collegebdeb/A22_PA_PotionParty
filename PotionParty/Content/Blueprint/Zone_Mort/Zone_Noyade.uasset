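; Drowning death zone that punishes a ThirdPersonCharacter entering its box and sends it back to a random player start.
; On overlap it calls the character's TakeDamage, disables input and waits through a short delay.
; Two nested random booleans then pick one of the first four PlayerStart actors found, and the character moves to that location before input is re-enabled.
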(event `self.Box.OnComponentBeginOverlap`
  (params (OverlappedComponent :type "PrimitiveComponent Object Reference") (OtherActor :type "Actor Object Reference") (OtherComp :type "PrimitiveComponent Object Reference") (OtherBodyIndex :type Integer) (bFromSweep :type Boolean) (SweepResult :type "HitResult Structure (by ref)"))
  (bind _asthird_person_character (cast `/Game/ThirdPersonBP/Blueprints/ThirdPersonCharacter` OtherActor))
  (`/Game/ThirdPersonBP/Blueprints/ThirdPersonCharacter.TakeDamage` _asthird_person_character)
  (`self.DisableInput` _asthird_person_character null)
  (`KismetSystemLibrary.Delay` 2.0)
  (bind _outactors (`GameplayStatics.GetAllActorsOfClass` "/Script/Engine.PlayerStart"))
  (if (`KismetMathLibrary.RandomBool`)
    (if (`KismetMathLibrary.RandomBool`)
      (bind _rootcomponent (`Actor.RootComponent` _asthird_person_character))
      (`SceneComponent.K2_SetWorldLocation` _rootcomponent (`self.K2_GetActorLocation` (`|GetArrayItem` _outactors)) false false)
      (else
        (`SceneComponent.K2_SetWorldLocation` _rootcomponent (`self.K2_GetActorLocation` (`|GetArrayItem` _outactors 1)) false false)))
    (elif (`KismetMathLibrary.RandomBool`)
      (`SceneComponent.K2_SetWorldLocation` _rootcomponent (`self.K2_GetActorLocation` (`|GetArrayItem` _outactors 2)) false false)
      (else
        (`SceneComponent.K2_SetWorldLocation` _rootcomponent (`self.K2_GetActorLocation` (`|GetArrayItem` _outactors 3)) false false))))
  (`self.EnableInput` _asthird_person_character null))

(fn `UserConstructionScript`)