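; Lava death zone that respawns a player who overlaps its Box trigger.
; A ThirdPersonCharacter takes damage and loses input for a short delay, while a GhostCharacter skips straight to the shared teleport step.
; Nested random booleans pick one of the first four PlayerStarts as the destination.
; The shared path then re-enables ThirdPersonCharacter input and calls ScoreIngame on BP_GameMode with that character's Index.
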(event `self.Box.OnComponentBeginOverlap`
  (params (OverlappedComponent :type "PrimitiveComponent Object Reference") (OtherActor :type "Actor Object Reference") (OtherComp :type "PrimitiveComponent Object Reference") (OtherBodyIndex :type Integer) (bFromSweep :type Boolean) (SweepResult :type "HitResult Structure (by ref)"))
  ;[1 1 1] Quand le joueur entre en contact avec la zone de noyade sa le fais respawn dans un des points de spawn du jeu
  (bind _asthird_person_character (cast `/Game/ThirdPersonBP/Blueprints/ThirdPersonCharacter` OtherActor)
    (:`then`
      (`/Game/ThirdPersonBP/Blueprints/ThirdPersonCharacter.TakeDamage` _asthird_person_character)
      (`self.DisableInput` _asthird_person_character null)
      (`KismetSystemLibrary.Delay` 0.5))
    (:`CastFailed`
      (bind _asghost_character (cast `/Game/ThirdPersonBP/Blueprints/GhostCharacter` OtherActor))))
  (bind _outactors (`GameplayStatics.GetAllActorsOfClass` "/Script/Engine.PlayerStart"))
  (if (`KismetMathLibrary.RandomBool`)
    (if (`KismetMathLibrary.RandomBool`)
      (bind _capsulecomponent (`Character.CapsuleComponent` _asthird_person_character))
      (`SceneComponent.K2_SetWorldLocation` _capsulecomponent (`self.K2_GetActorLocation` (`|GetArrayItem` _outactors)) false false)
      (`SceneComponent.K2_SetWorldLocation` (`Character.CapsuleComponent` _asghost_character) (`self.K2_GetActorLocation` (`|GetArrayItem` _outactors)) false false)
      (else
        (`SceneComponent.K2_SetWorldLocation` _capsulecomponent (`self.K2_GetActorLocation` (`|GetArrayItem` _outactors 1)) false false)
        (`SceneComponent.K2_SetWorldLocation` (`Character.CapsuleComponent` _asghost_character) (`self.K2_GetActorLocation` (`|GetArrayItem` _outactors 1)) false false)))
    (elif (`KismetMathLibrary.RandomBool`)
      (`SceneComponent.K2_SetWorldLocation` _capsulecomponent (`self.K2_GetActorLocation` (`|GetArrayItem` _outactors 2)) false false)
      (`SceneComponent.K2_SetWorldLocation` (`Character.CapsuleComponent` _asghost_character) (`self.K2_GetActorLocation` (`|GetArrayItem` _outactors 2)) false false)
      (else
        (`SceneComponent.K2_SetWorldLocation` _capsulecomponent (`self.K2_GetActorLocation` (`|GetArrayItem` _outactors 3)) false false)
        (`SceneComponent.K2_SetWorldLocation` (`Character.CapsuleComponent` _asghost_character) (`self.K2_GetActorLocation` (`|GetArrayItem` _outactors 3)) false false))))
  (`self.EnableInput` _asthird_person_character null)
  (bind _asbp_game_mode (cast `/Game/Blueprint/BP_GameMode` (`GameplayStatics.GetGameMode`)))
  (`/Game/Blueprint/BP_GameMode.Score_ingame-` _asbp_game_mode (`/Game/ThirdPersonBP/Blueprints/ThirdPersonCharacter.Index` _asthird_person_character)))

(fn `UserConstructionScript`)