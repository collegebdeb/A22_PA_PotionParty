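; Short-lived explosion zone actor that damages characters and spawns an explosive ghost AI.
; On BeginPlay it adds a Niagara effect, plays a blast sound, spawns BP_IA_fantome_Explosive at a random point within the Box extent, then destroys itself after one second.
; Sphere overlaps call TakeDamage on any ThirdPersonCharacter whose Index differs from the zone's.
; The GetIndex event has an empty body.
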(event `self.ReceiveBeginPlay`
  ;[1 1 1] fait apparaitre un fantome puis fais disparaitre la zone d'explosion après 1 seconde
  (`AddComponent|NODE_AddNiagaraComponent-0`)
  (`GameplayStatics.PlaySound2D` "/Game/Sound/SFX_Potion/P_Explo/SFX_ExplosionBlast3_Cue.SFX_ExplosionBlast3_Cue" 1.0 1.0 0.0 null null)
  (`AIBlueprintHelperLibrary.SpawnAIFromClass` "/Game/ThirdPersonBP/IA/BP_IA_fantome_Explosive.BP_IA_fantome_Explosive_C" null (`KismetMathLibrary.RandomPointInBoundingBox` (`SceneComponent.K2_GetComponentLocation` (`self.DefaultSceneRoot`)) (`BoxComponent.BoxExtent` (`self.Box`))) (struct) false null)
  (`KismetSystemLibrary.Delay` 1.0)
  (`self.K2_DestroyActor`))

(event `self.Sphere.OnComponentBeginOverlap`
  (params (OverlappedComponent :type "PrimitiveComponent Object Reference") (OtherActor :type "Actor Object Reference") (OtherComp :type "PrimitiveComponent Object Reference") (OtherBodyIndex :type Integer) (bFromSweep :type Boolean) (SweepResult :type "HitResult Structure (by ref)"))
  ;[1 1 1] Inflige 1 de domage
  (bind _asthird_person_character (cast `/Game/ThirdPersonBP/Blueprints/ThirdPersonCharacter` OtherActor))
  (if (not (== (`/Game/ThirdPersonBP/Blueprints/ThirdPersonCharacter.Index` _asthird_person_character) (stale `GetIndex` Index)))
    (`/Game/ThirdPersonBP/Blueprints/ThirdPersonCharacter.TakeDamage` _asthird_person_character)))

(event `GetIndex`
  (params (Index :type Integer)))

(fn `UserConstructionScript`)