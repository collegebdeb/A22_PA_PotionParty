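; BP_Zone_Transformation is a short-lived potion area that transforms players caught in it, per its comments into a rat for a limited time.
; On spawn it plays a sound, scales its sphere up with the PotionRadius timeline and destroys itself after a one-second delay.
; After a brief delay, overlapping ThirdPersonCharacters with a different Index get TransfoToucher called, and BP_GameMode's ScoreIngame receives the zone's Index.
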(event `self.ReceiveBeginPlay`
  ;[1 1 1] Au bout de 1.5 seconde fais disparaitre la zone de transformation
  (`GameplayStatics.PlaySound2D` "/Game/Sound/SFX_Potion/P_Meta/SFX_MagicalShimmer_Cue.SFX_MagicalShimmer_Cue" 1.0 1.0 0.0 null null)
  (bind (_direction _newtrack_0) (`Timeline|PotionRadius`)
    (:`Update`
      (`SceneComponent.SetRelativeScale3D` (`self.Sphere`) (`KismetMathLibrary.VLerp` (0.0 0.0 0.0) (1.0 1.0 1.0) _newtrack_0))
      (`KismetSystemLibrary.Delay` 1.0)
      (`self.K2_DestroyActor`))))

(event `self.Sphere.OnComponentBeginOverlap`
  (params (OverlappedComponent :type "PrimitiveComponent Object Reference") (OtherActor :type "Actor Object Reference") (OtherComp :type "PrimitiveComponent Object Reference") (OtherBodyIndex :type Integer) (bFromSweep :type Boolean) (SweepResult :type "HitResult Structure (by ref)"))
  ;[1 1 1] Transforme le joueur en rat pour 10 seconde et retransforme le par la suite en humain
  (`KismetSystemLibrary.Delay` 0.2)
  (bind _asthird_person_character (cast `/Game/ThirdPersonBP/Blueprints/ThirdPersonCharacter` OtherActor))
  (if (not (== (`/Game/ThirdPersonBP/Blueprints/ThirdPersonCharacter.Index` _asthird_person_character) (stale `GetIndex` Index)))
    (`GameplayStatics.PlaySound2D` "/Game/Sound/SFX_Interactivity/TransformRat/SFX_SqueezeCondiment_Cue.SFX_SqueezeCondiment_Cue" 1.0 1.0 0.0 null null)
    (`/Game/ThirdPersonBP/Blueprints/ThirdPersonCharacter.transfo toucher` _asthird_person_character)
    (bind _asbp_game_mode (cast `/Game/Blueprint/BP_GameMode` (`GameplayStatics.GetGameMode`)))
    (`/Game/Blueprint/BP_GameMode.Score_ingame+` _asbp_game_mode (stale `GetIndex` Index))))

(event `GetIndex`
  (params (Index :type Integer))
  ;[1 1 1] Transforme le joueur en rat pour 10 seconde et retransforme le par la suite en humain
)

(fn `UserConstructionScript`)