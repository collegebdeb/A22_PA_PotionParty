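; BP_Champignon_sol is a physics-driven mushroom pickup that adds to a ThirdPersonCharacter's Champignon count.
; The ChampignonSol event launches it along the actor's forward vector, then sets collision from the indexed player's IngrLoin flag: query and physics if true, physics only otherwise.
; Pickup relies on the Hit event rather than overlap: a hit with a ThirdPersonCharacter increments its counter and destroys the mushroom.
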(event `self.ReceiveBeginPlay`)

(event `ChampignonSol`
  (params (index :type Integer))
  (`PrimitiveComponent.SetPhysicsLinearVelocity` (`self.champignon`) (* (`self.GetActorForwardVector`) 500.0) false "None")
  (bind _asthird_person_character (cast `/Game/ThirdPersonBP/Blueprints/ThirdPersonCharacter` (`GameplayStatics.GetPlayerPawn` index)))
  (if (`/Game/ThirdPersonBP/Blueprints/ThirdPersonCharacter.ingrLoin` _asthird_person_character)
    (`PrimitiveComponent.SetCollisionEnabled` (`self.champignon`) "QueryAndPhysics")
    (else
      (`PrimitiveComponent.SetCollisionEnabled` (`self.champignon`) "PhysicsOnly"))))

(event `self.ReceiveActorBeginOverlap`
  (params (OtherActor :type "Actor Object Reference")))

(event `self.ReceiveHit`
  (params (MyComp :type "PrimitiveComponent Object Reference") (Other :type "Actor Object Reference") (OtherComp :type "PrimitiveComponent Object Reference") (bSelfMoved :type Boolean) (HitLocation :type "Vector Structure") (HitNormal :type "Vector Structure") (NormalImpulse :type "Vector Structure") (Hit :type "HitResult Structure (by ref)"))
  (bind _asthird_person_character (cast `/Game/ThirdPersonBP/Blueprints/ThirdPersonCharacter` Other))
  (set `/Game/ThirdPersonBP/Blueprints/ThirdPersonCharacter.Champignon` (+ (`/Game/ThirdPersonBP/Blueprints/ThirdPersonCharacter.Champignon` _asthird_person_character) 1) _asthird_person_character)
  (`self.K2_DestroyActor`))

(fn `UserConstructionScript`)