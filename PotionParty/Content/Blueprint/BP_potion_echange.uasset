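; Thrown exchange potion that spawns an exchange effect zone where it hits, carrying the thrower's ingredient inventory.
; PotionEchange looks up the thrower by player index, prints their four ingredient counts and enables query collision only if PotionAssezLoin is set, avoiding detonation on the thrower.
; On hit, it spawns BP_Zone_Echange, passes it those counts and the index through EchangeActif, then destroys itself.
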(event `PotionEchange`
  (params (index :type Integer))
  ;[1 1 1] Quand la potion est lancer empêche qu'elle explose au contacte du joueur pendant 0.5 secondes et on affiche les items du joueur qui lance la potion
  (bind _asthird_person_character (cast `/Game/ThirdPersonBP/Blueprints/ThirdPersonCharacter` (`GameplayStatics.GetPlayerPawn` index)))
  (`KismetSystemLibrary.PrintString` (`KismetStringLibrary.Concat_StrStr` "Baie : " (`KismetStringLibrary.Conv_IntToString` (`/Game/ThirdPersonBP/Blueprints/ThirdPersonCharacter.Baie` _asthird_person_character)) " Champignon : " (`KismetStringLibrary.Conv_IntToString` (`/Game/ThirdPersonBP/Blueprints/ThirdPersonCharacter.Champignon` _asthird_person_character)) " Queue de rat : " (`KismetStringLibrary.Conv_IntToString` (`/Game/ThirdPersonBP/Blueprints/ThirdPersonCharacter.QueueDeRat` _asthird_person_character)) " Ectoplasme : " (`KismetStringLibrary.Conv_IntToString` (`/Game/ThirdPersonBP/Blueprints/ThirdPersonCharacter.Ectoplasme` _asthird_person_character))))
  (if (`/Game/ThirdPersonBP/Blueprints/ThirdPersonCharacter.PotionAssezLoin` _asthird_person_character)
    (`PrimitiveComponent.SetCollisionEnabled` (`self.potionEchenge`) "QueryAndPhysics")
    (else
      (`PrimitiveComponent.SetCollisionEnabled` (`self.potionEchenge`) "PhysicsOnly"))))

(event `self.ReceiveHit`
  (params (MyComp :type "PrimitiveComponent Object Reference") (Other :type "Actor Object Reference") (OtherComp :type "PrimitiveComponent Object Reference") (bSelfMoved :type Boolean) (HitLocation :type "Vector Structure") (HitNormal :type "Vector Structure") (NormalImpulse :type "Vector Structure") (Hit :type "HitResult Structure (by ref)"))
  ;[1 1 1] quand l'objet touche quelque chose il génère la zone d'effet et envoie les info du lanceur pour l'inventaire
  (bind _returnvalue (`|SpawnActorFromClass` "/Game/Blueprint/BP_Zone_Echange.BP_Zone_Echange_C" (`KismetMathLibrary.MakeTransform` (`SceneComponent.K2_GetComponentLocation` (`self.potionEchenge`))) "Undefined" "OverrideRootScale" null null))
  (`/Game/Blueprint/BP_Zone_Echange.EchangeActif` _returnvalue (`/Game/ThirdPersonBP/Blueprints/ThirdPersonCharacter.Baie` (stale `PotionEchange` _asthird_person_character)) (`/Game/ThirdPersonBP/Blueprints/ThirdPersonCharacter.Champignon` (stale `PotionEchange` _asthird_person_character)) (`/Game/ThirdPersonBP/Blueprints/ThirdPersonCharacter.QueueDeRat` (stale `PotionEchange` _asthird_person_character)) (`/Game/ThirdPersonBP/Blueprints/ThirdPersonCharacter.Ectoplasme` (stale `PotionEchange` _asthird_person_character)) (stale `PotionEchange` index))
  (`self.K2_DestroyActor`))

(fn `UserConstructionScript`)