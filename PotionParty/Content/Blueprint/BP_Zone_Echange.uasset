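; BP_Zone_Echange is a short-lived "exchange" zone actor that destroys itself one second after spawning.
; After a brief delay, Sphere begin and end overlaps share one path that compares character indices with its own Index.
; On a mismatch, it plays an impact sound, then calls Stun and ToucherParEchange on the ThirdPersonCharacter.
; The ingredient-inventory swap and switch limit are disconnected, and GetIndex and EchangeActif events are empty.
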(event `self.ReceiveBeginPlay`
  ;[1 1 1] on détruit la zone après un certain temps
  (`KismetSystemLibrary.Delay` 1.0)
  (`self.K2_DestroyActor`))

(event `self.Sphere.OnComponentBeginOverlap`
  (params (OverlappedComponent :type "PrimitiveComponent Object Reference") (OtherActor :type "Actor Object Reference") (OtherComp :type "PrimitiveComponent Object Reference") (OtherBodyIndex :type Integer) (bFromSweep :type Boolean) (SweepResult :type "HitResult Structure (by ref)"))
  (`KismetSystemLibrary.Delay` 0.1)
  ;[1 1 1] on donne la valeur de l'inventaire du lanceur à la personne toucher
  (bind _asthird_person_character (cast `/Game/ThirdPersonBP/Blueprints/ThirdPersonCharacter` OtherActor))
  (if (not (or (== (`/Game/ThirdPersonBP/Blueprints/ThirdPersonCharacter.Index` _asthird_person_character) (stale `GetIndex` Index)) (== (`/Game/ThirdPersonBP/Blueprints/ThirdPersonCharacter.Index` (stale `self.Sphere.OnComponentEndOverlap` _asthird_person_character)) (stale `GetIndex` Index)))) :!label _label
    (`GameplayStatics.PlaySound2D` "/Game/Sound/SFX_Potion/P_Exchange/SFX_ComicHeadImpact_Cue.SFX_ComicHeadImpact_Cue" 1.0 1.0 0.0 null null)
    (`/Game/ThirdPersonBP/Blueprints/ThirdPersonCharacter.Stun` _asthird_person_character)
    (`/Game/ThirdPersonBP/Blueprints/ThirdPersonCharacter.toucherParEchange` _asthird_person_character)))

(event `GetIndex`
  (params (Index :type Integer)))

(event `self.Sphere.OnComponentEndOverlap`
  (params (OverlappedComponent :type "PrimitiveComponent Object Reference") (OtherActor :type "Actor Object Reference") (OtherComp :type "PrimitiveComponent Object Reference") (OtherBodyIndex :type Integer))
  (`KismetSystemLibrary.Delay` 0.1)
  (bind _asthird_person_character (cast `/Game/ThirdPersonBP/Blueprints/ThirdPersonCharacter` OtherActor))
  (goto _label))

(event `EchangeActif`
  (params (BaieLanceur :type Integer) (ChampignonLanceur :type Integer) (RatLanceur :type Integer) (EctoplasmeLanceur :type Integer) (Index :type Integer)))

(fn `UserConstructionScript`)