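; Zone actor that temporarily changes the appearance of a ThirdPersonCharacter that enters its sphere.
; On sphere overlap it swaps the character's skeletal mesh and anim class to the mannequin set, then switches both to the wizard set after a timed delay.
; BeginPlay disables the sphere's collision after a short delay and never re-enables it, with debug prints marking the steps.
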(event `self.ReceiveBeginPlay`
  (`KismetSystemLibrary.Delay` 1.5)
  (`KismetSystemLibrary.PrintString` "Transformation")
  (`PrimitiveComponent.SetCollisionEnabled` (`self.Sphere`) "NoCollision")
  (`KismetSystemLibrary.Delay` 10.0))

(event `self.Sphere.OnComponentBeginOverlap`
  (params (OverlappedComponent :type "PrimitiveComponent Object Reference") (OtherActor :type "Actor Object Reference") (OtherComp :type "PrimitiveComponent Object Reference") (OtherBodyIndex :type Integer) (bFromSweep :type Boolean) (SweepResult :type "HitResult Structure (by ref)"))
  (bind _asthird_person_character (cast `/Game/ThirdPersonBP/Blueprints/ThirdPersonCharacter` OtherActor))
  (bind _mesh (`Character.Mesh` _asthird_person_character))
  (`SkinnedMeshComponent.SetSkinnedAssetAndUpdate` _mesh "/Game/Mannequin/Character/Mesh/SK_Mannequin.SK_Mannequin" true)
  (`SkeletalMeshComponent.SetAnimInstanceClass` _mesh "/Game/BattleWizardPolyart/Animations/ThirdPerson_AnimBP.ThirdPerson_AnimBP_C")
  (`KismetSystemLibrary.PrintString` "detransform")
  (`KismetSystemLibrary.Delay` 10.0)
  (`SkinnedMeshComponent.SetSkinnedAssetAndUpdate` _mesh "/Game/BattleWizardPolyart/Meshes/WizardSM.WizardSM" true)
  (`SkeletalMeshComponent.SetAnimInstanceClass` _mesh "/Game/BattleWizardPolyart/Animations/ThirdPerson_AnimBP1.ThirdPerson_AnimBP1_C"))

(fn `UserConstructionScript`)