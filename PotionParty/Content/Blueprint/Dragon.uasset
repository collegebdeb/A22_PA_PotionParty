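; Dragon actor that periodically sweeps a damaging sphere along a spline path as a recurring hazard.
; Tick drives a DoOnce that, after a configurable delay, activates Niagara, plays a camera shake at the ShakePoint actor and starts a timeline.
; The timeline moves the sphere along the spline, and its update starts a 60-second delay that resets the DoOnce.
; Sphere overlap calls TakeDamage on the ThirdPersonCharacter.
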(event `self.ReceiveTick`
  (params (DeltaSeconds :type "Float (single-precision)"))
  (`/Engine/EditorBlueprintResources/StandardMacros.DoOnce` false :!label _label
    (:`Completed`
      (`KismetSystemLibrary.Delay` (`self.Duration`))
      (`ActorComponent.Activate` (`self.Niagara`) false)
      (bind _returnvalue (`GameplayStatics.GetActorOfClass` "/Game/Blueprint/ShakePoint.ShakePoint_C"))
      (`GameplayStatics.PlayWorldCameraShake` "/Game/Blueprint/Dragon_shake.Dragon_shake_C" (`self.K2_GetActorLocation` _returnvalue) 0.0 1.0 1000000000.0)
      (bind (_direction _newtrack_0) (`Timeline|Timeline_0` :!via `PlayFromStart`)
        (:`Update`
          (`SceneComponent.K2_SetWorldLocation` (`self.Sphere`) (`SplineComponent.GetLocationAtDistanceAlongSpline` (`self.Spline`) (* (`SplineComponent.GetSplineLength` (`self.Spline`)) _newtrack_0) "World") false false)
          (`KismetSystemLibrary.Delay` 60.0)
          (goto _label :!via `Reset`))))))

(event `self.ReceiveBeginPlay`)

(event `self.Sphere.OnComponentBeginOverlap`
  (params (OverlappedComponent :type "PrimitiveComponent Object Reference") (OtherActor :type "Actor Object Reference") (OtherComp :type "PrimitiveComponent Object Reference") (OtherBodyIndex :type Integer) (bFromSweep :type Boolean) (SweepResult :type "HitResult Structure (by ref)"))
  (bind _asthird_person_character (cast `/Game/ThirdPersonBP/Blueprints/ThirdPersonCharacter` OtherActor))
  (`/Game/ThirdPersonBP/Blueprints/ThirdPersonCharacter.TakeDamage` _asthird_person_character))

(fn `UserConstructionScript`)