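; MyLibrary is a Blueprint library with DropItem, which places an actor at a location and snaps it to a surface.
; It moves the actor there, then line traces on Visibility, though the end offset is zero as written.
; On a hit, it teleports the actor to the hit point and faces it along the forward vector, optionally aligning up to the surface normal.
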(fn `DropItem`
  (params (Actor :type "Actor Object Reference") (Location :type "Vector Structure") (ForwardVector :type "Vector Structure") (AlingWithGround :type Boolean))
  (bind _location (`local.Location`))
  (bind _forwardvector (`local.ForwardVector`))
  (`Actor.K2_SetActorLocation` Actor Location false false)
  (bind (_outhit _returnvalue) (`KismetSystemLibrary.LineTraceSingle` null _location (- _location (0.0 0.0 0.0)) "TraceTypeQuery1"))
  (if _returnvalue
    (bind (_bblockinghit _binitialoverlap _time _distance _location_2 _impactpoint _normal _impactnormal) (`GameplayStatics.BreakHitResult` _outhit))
    (`Actor.K2_SetActorLocation` (`local.Actor`) _location_2 false true)
    (if (`local.AlingWithGround`)
      (`Actor.K2_SetActorRotation` (`local.Actor`) (`KismetMathLibrary.MakeRotFromZX` _impactnormal _forwardvector) false)
      (else
        (`Actor.K2_SetActorRotation` (`local.Actor`) (`KismetMathLibrary.MakeRotFromX` _forwardvector) false)))))