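; Ectoplasm ground item that a ThirdPersonCharacter collects on contact, adding one to its Ectoplasme count, and that despawns after 15 seconds.
; The EctoplasmeSol event launches it forward through physics velocity, then picks query-and-physics or physics-only collision from the indexed player's IngrLoin flag.
; Hit handles pickup with destruction and a sound, plus a one-time body-fall sound on first impact.
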(event `self.ReceiveBeginPlay`
  (`KismetSystemLibrary.Delay` 15.0)
  (`self.K2_DestroyActor`))

(event `EctoplasmeSol`
  (params (Index :type Integer))
  (`PrimitiveComponent.SetPhysicsLinearVelocity` (`self.ectoplasme`) (* (`self.GetActorForwardVector`) 500.0) false "None")
  (bind _asthird_person_character (cast `/Game/ThirdPersonBP/Blueprints/ThirdPersonCharacter` (`GameplayStatics.GetPlayerPawn` Index)))
  (if (`/Game/ThirdPersonBP/Blueprints/ThirdPersonCharacter.ingrLoin` _asthird_person_character)
    (`PrimitiveComponent.SetCollisionEnabled` (`self.ectoplasme`) "QueryAndPhysics")
    (else
      (`PrimitiveComponent.SetCollisionEnabled` (`self.ectoplasme`) "PhysicsOnly"))))

(event `self.ReceiveHit`
  (params (MyComp :type "PrimitiveComponent Object Reference") (Other :type "Actor Object Reference") (OtherComp :type "PrimitiveComponent Object Reference") (bSelfMoved :type Boolean) (HitLocation :type "Vector Structure") (HitNormal :type "Vector Structure") (NormalImpulse :type "Vector Structure") (Hit :type "HitResult Structure (by ref)"))
  (`|ExecutionSequence`
    (:`then_0`
      (bind _asthird_person_character (cast `/Game/ThirdPersonBP/Blueprints/ThirdPersonCharacter` Other))
      (set `/Game/ThirdPersonBP/Blueprints/ThirdPersonCharacter.Ectoplasme` (+ (`/Game/ThirdPersonBP/Blueprints/ThirdPersonCharacter.Ectoplasme` _asthird_person_character) 1) _asthird_person_character)
      (`self.K2_DestroyActor`)
      (`GameplayStatics.PlaySound2D` "/Game/Sound/SFX_Interactivity/ItemOnFloor/FloorItem_Cue.FloorItem_Cue" 1.0 1.0 0.0 null null))
    (:`then_1`
      (`/Engine/EditorBlueprintResources/StandardMacros.DoOnce` false
        (:`Completed`
          (`GameplayStatics.PlaySound2D` "/Game/Sound/SFX_Interactivity/FallOnFloor/SFX_DonkeyBodyFall_Cue.SFX_DonkeyBodyFall_Cue" 1.0 1.0 0.0 null null))))))

(event `self.ReceiveActorBeginOverlap`
  (params (OtherActor :type "Actor Object Reference")))

(fn `UserConstructionScript`)