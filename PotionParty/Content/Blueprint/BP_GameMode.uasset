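; Game mode for a local multiplayer last-player-standing game that loads a random one of four levels when one character remains.
; On BeginPlay it creates a local player per PlayerStart, ordered by integer PlayerStartTag, each possessing a spawned BP_InputReceiver.
; SpawnPlayer later spawns a ThirdPersonCharacter at a receiver's transform and hands that player's controller to it.
; CharacterDeath counts survivors as existing characters minus one to trigger the level change.
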(event `self.ReceiveBeginPlay`
  (`self.GetPlayerStartPoint`)
  (`self.SpawnInputReceiver`))

(event `CharacterDeath`
  (bind _outactors (`GameplayStatics.GetAllActorsOfClass` "/Game/ThirdPersonBP/Blueprints/ThirdPersonCharacter.ThirdPersonCharacter_C"))
  (bind _output_get (set `self.NumberOfPlayerAlive` (+ (`KismetArrayLibrary.Array_Length` _outactors) -1)))
  (if (== _output_get 1)
    (`GameplayStatics.OpenLevel` (`KismetArrayLibrary.Array_Random` (`|MakeArray` (`self.Waterfall_Main`) (`self.Mountain_Main`) (`self.Library_Main`) (`self.Joustng_Main`))))))

(fn `GetPlayerStartPoint`
  (bind _outactors (`GameplayStatics.GetAllActorsOfClass` "/Script/Engine.PlayerStart"))
  (set `self.PlayerStartArray` _outactors))

(fn `NameToInt`
  (params (PlayerStart :type "PlayerStart Object Reference"))
  (returns (ReturnValue :type Integer))
  (return (`KismetStringLibrary.Conv_StringToInt` (`KismetStringLibrary.Conv_NameToString` (`PlayerStart.PlayerStartTag` PlayerStart)))))

(fn `SpawnInputReceiver`
  (locals (Index :type Integer))
  (bind _returnvalue (`GameplayStatics.GetPlayerController` (`local.Index`)))
  (for (_ _array_index) (`self.PlayerStartArray`)
    (set `local.Index` _array_index)
    (for _array_element (`self.PlayerStartArray`)
      (if (== (`self.NameToInt` _array_element) (`local.Index`))
        (`GameplayStatics.CreatePlayer` -1)
        (bind _returnvalue_2 (`|SpawnActorFromClass` "/Game/Blueprint/BP_InputReceiver.BP_InputReceiver_C" (`self.GetTransform` (`|GetArrayItem` (`self.PlayerStartArray`) (`local.Index`))) "Undefined" "OverrideRootScale" null (`local.Index`) null))
        (`KismetArrayLibrary.Array_AddUnique` (`self.playerInputReceiverArray`) _returnvalue_2)
        (`Controller.Possess` _returnvalue _returnvalue_2)
        (`KismetArrayLibrary.Array_AddUnique` (`self.PlayerControllerArray`) _returnvalue)))))

(fn `SpawnPlayer`
  (params (CurrentPlayerIndex :type Integer) (InputReceiver :type "/Game/Blueprint/BP_InputReceiver Object Reference"))
  (returns (return :type Boolean))
  (bind _returnvalue (`|SpawnActorFromClass` "/Game/ThirdPersonBP/Blueprints/ThirdPersonCharacter.ThirdPersonCharacter_C" (`self.GetTransform` (`local.InputReceiver`)) "Undefined" "OverrideRootScale" null (`local.CurrentPlayerIndex`) null))
  (`Controller.Possess` (`GameplayStatics.GetPlayerController` (`local.CurrentPlayerIndex`)) _returnvalue)
  (return false))

(fn `UserConstructionScript`)