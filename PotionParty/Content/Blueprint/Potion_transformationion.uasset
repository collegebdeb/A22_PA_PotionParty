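; Thrown transformation potion that spawns a Zone_Transformation actor at its sphere's location on hit, then destroys itself.
; A custom event looks up the player pawn by index as a ThirdPersonCharacter and reads its PotionAssezLoin flag.
; That flag switches the sphere between physics-only and query-and-physics collision, meant to stop the potion exploding on the player just after the throw.
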(event `PotionTransmormation`
  (params (index :type Integer))
  ;[1 1 1] Quand la potion est lancer empêche qu'elle explose au contacte du joueur pendant 0.5 secondes
  (bind _asthird_person_character (cast `/Game/ThirdPersonBP/Blueprints/ThirdPersonCharacter` (`GameplayStatics.GetPlayerPawn` index)))
  (if (`/Game/ThirdPersonBP/Blueprints/ThirdPersonCharacter.PotionAssezLoin` _asthird_person_character)
    (`PrimitiveComponent.SetCollisionEnabled` (`self.Sphere`) "QueryAndPhysics")
    (else
      (`PrimitiveComponent.SetCollisionEnabled` (`self.Sphere`) "PhysicsOnly"))))

(event `self.ReceiveHit`
  (params (MyComp :type "PrimitiveComponent Object Reference") (Other :type "Actor Object Reference") (OtherComp :type "PrimitiveComponent Object Reference") (bSelfMoved :type Boolean) (HitLocation :type "Vector Structure") (HitNormal :type "Vector Structure") (NormalImpulse :type "Vector Structure") (Hit :type "HitResult Structure (by ref)"))
  (`|SpawnActorFromClass` "/Game/Blueprint/Zone_Transformation.Zone_Transformation_C" (`KismetMathLibrary.MakeTransform` (`SceneComponent.K2_GetComponentLocation` (`self.Sphere`))) "Undefined" "OverrideRootScale" null null)
  (`self.K2_DestroyActor`))

(fn `UserConstructionScript`)