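; Rat-tail item on the ground that the third-person character collects, adding one to its QueueDeRat count.
; The QueueSol event launches the tail along the actor's forward vector, then reads the indexed player's IngrLoin flag to choose between query-and-physics and physics-only collision.
; Pickup runs on Hit rather than overlap: a hit with the character increments the count and destroys the actor.
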(event `QueueSol`
  (params (Index :type Integer))
  (`PrimitiveComponent.SetPhysicsLinearVelocity` (`self.queue de rat`) (* (`self.GetActorForwardVector`) 1000.0) false "None")
  (bind _asthird_person_character (cast `/Game/ThirdPersonBP/Blueprints/ThirdPersonCharacter` (`GameplayStatics.GetPlayerPawn` Index)))
  (if (`/Game/ThirdPersonBP/Blueprints/ThirdPersonCharacter.ingrLoin` _asthird_person_character)
    (`PrimitiveComponent.SetCollisionEnabled` (`self.queue de rat`) "QueryAndPhysics")
    (else
      (`PrimitiveComponent.SetCollisionEnabled` (`self.queue de rat`) "PhysicsOnly"))))

(event `self.ReceiveActorBeginOverlap`
  (params (OtherActor :type "Actor Object Reference")))

(event `self.ReceiveHit`
  (params (MyComp :type "PrimitiveComponent Object Reference") (Other :type "Actor Object Reference") (OtherComp :type "PrimitiveComponent Object Reference") (bSelfMoved :type Boolean) (HitLocation :type "Vector Structure") (HitNormal :type "Vector Structure") (NormalImpulse :type "Vector Structure") (Hit :type "HitResult Structure (by ref)"))
  (bind _asthird_person_character (cast `/Game/ThirdPersonBP/Blueprints/ThirdPersonCharacter` Other))
  (set `/Game/ThirdPersonBP/Blueprints/ThirdPersonCharacter.QueueDeRat` (+ (`/Game/ThirdPersonBP/Blueprints/ThirdPersonCharacter.QueueDeRat` _asthird_person_character) 1) _asthird_person_character)
  (`self.K2_DestroyActor`))

(fn `UserConstructionScript`)