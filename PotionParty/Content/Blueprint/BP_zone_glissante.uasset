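; BP_zone_glissante is a temporary slippery patch that makes other players fall and costs them a life.
; On spawn it plays a sound, stops its particles after a short delay, then destroys itself fifteen seconds later.
; Box overlap plays a fall montage on any ThirdPersonCharacter whose Index differs from the zone's.
; If the victim can take damage, it applies damage and calls ScoreIngame on BP_GameMode with the zone's Index.
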(event `self.ReceiveBeginPlay`
  ;[1 1 1] au bout de 15 secondes la tache disparait
  (`GameplayStatics.PlaySound2D` "/Game/Sound/SFX_Potion/P_Glis/SFX_TentaclesRetract6_Cue.SFX_TentaclesRetract6_Cue" 1.0 1.0 0.0 null null)
  (`KismetSystemLibrary.Delay` 2.0)
  (`ActorComponent.Deactivate` (`self.ParticleSystem`))
  (`KismetSystemLibrary.Delay` 15.0)
  (`self.K2_DestroyActor`))

(event `self.ReceiveTick`
  (params (DeltaSeconds :type "Float (single-precision)")))

(event `self.Box.OnComponentBeginOverlap`
  (params (OverlappedComponent :type "PrimitiveComponent Object Reference") (OtherActor :type "Actor Object Reference") (OtherComp :type "PrimitiveComponent Object Reference") (OtherBodyIndex :type Integer) (bFromSweep :type Boolean) (SweepResult :type "HitResult Structure (by ref)"))
  ;[1 1 1] Fait glisser le personnage et lui enlève une vie
  (bind _asthird_person_character (cast `/Game/ThirdPersonBP/Blueprints/ThirdPersonCharacter` OtherActor))
  (if (not (== (`/Game/ThirdPersonBP/Blueprints/ThirdPersonCharacter.Index` _asthird_person_character) (stale `GetIndex` Index)))
    (`GameplayStatics.PlaySound2D` "/Game/Sound/SFX_Interactivity/SlipBreakBack/SFX_BubbleBlips_Cue.SFX_BubbleBlips_Cue" 1.0 1.0 0.0 null null)
    (`Character.PlayAnimMontage` _asthird_person_character "/Game/ThirdPersonBP/Animation/SweepFall4UE4_Montage.SweepFall4UE4_Montage" 1.0 "Start")
    (if (`/Game/ThirdPersonBP/Blueprints/ThirdPersonCharacter.CanTakeDamage` _asthird_person_character)
      (`/Game/ThirdPersonBP/Blueprints/ThirdPersonCharacter.TakeDamage` _asthird_person_character)
      (bind _asbp_game_mode (cast `/Game/Blueprint/BP_GameMode` (`GameplayStatics.GetGameMode`)))
      (`/Game/Blueprint/BP_GameMode.Score_ingame+` _asbp_game_mode (stale `GetIndex` Index)))))

(event `GetIndex`
  (params (Index :type Integer)))

(fn `UserConstructionScript`)