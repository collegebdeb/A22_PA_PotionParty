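; Berry ("Baie") pickup actor that is thrown with physics and can be collected by the third-person character.
; The baieSol event launches the berry along the actor's forward vector, then reads IngrLoin on the given player's character to enable query-and-physics or physics-only collision.
; When a ThirdPersonCharacter overlaps the actor, that character's Baie count goes up by one and the pickup destroys itself.
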(event `self.ReceiveBeginPlay`)

(event `baieSol`
  (params (Index :type Integer))
  (`PrimitiveComponent.SetPhysicsLinearVelocity` (`self.Baie`) (* (`self.GetActorForwardVector`) 1000.0) false "None")
  (bind _asthird_person_character (cast `/Game/ThirdPersonBP/Blueprints/ThirdPersonCharacter` (`GameplayStatics.GetPlayerPawn` Index)))
  (if (`/Game/ThirdPersonBP/Blueprints/ThirdPersonCharacter.ingrLoin` _asthird_person_character)
    (`PrimitiveComponent.SetCollisionEnabled` (`self.Baie`) "QueryAndPhysics")
    (else
      (`PrimitiveComponent.SetCollisionEnabled` (`self.Baie`) "PhysicsOnly"))))

(event `self.ReceiveActorBeginOverlap`
  (params (OtherActor :type "Actor Object Reference"))
  (bind _asthird_person_character (cast `/Game/ThirdPersonBP/Blueprints/ThirdPersonCharacter` OtherActor))
  (set `/Game/ThirdPersonBP/Blueprints/ThirdPersonCharacter.Baie` (+ (`/Game/ThirdPersonBP/Blueprints/ThirdPersonCharacter.Baie` _asthird_person_character) 1) _asthird_person_character)
  (`self.K2_DestroyActor`))

(fn `UserConstructionScript`)